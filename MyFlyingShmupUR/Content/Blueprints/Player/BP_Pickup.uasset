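; BP_Pickup is a collectible actor that passes stat and weapon upgrade values to whatever actor overlaps it.
; On overlap it sends its health, lives, enemy damage and shooting variables to that actor through an OnCollectPickUpMessage call, with no type check or filter.
; It then spawns a BP_Pickup_Effect, attaches it to the overlapping actor and destroys itself.
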(event `self.ReceiveActorBeginOverlap`
  (params (OtherActor :type "Actor Object Reference"))
  (message `/Game/Core/BPI_MyFlyingShmup.OnCollectPickUp` OtherActor (`self.MaxHealth`) (`self.Health`) (`self.Lives`) (`self.GlobalEnemyDamage`) (`self.RateOfFire`) (`self.ShootingDirection`) (`self.HasTopGuns`) (`self.BulletsToShoot`))
  (bind _returnvalue (`|SpawnActorFromClass` "/Game/Particles/BP_Pickup_Effect.BP_Pickup_Effect_C" (`KismetMathLibrary.MakeTransform` (0.0 0.0 0.0)) "Undefined" "MultiplyWithRoot" null null))
  (`self.K2_AttachToActor` _returnvalue OtherActor "None" "KeepRelative" "KeepRelative" "KeepRelative" false)
  (`self.K2_DestroyActor`))

(fn `UserConstructionScript`)