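; Player ship pawn for a flying shmup, with Y/Z movement, mesh tilt and brief collision-free spawn protection.
; Firing reads burst, spread and rate from the player controller, spawning bullets from twin guns plus timed top guns.
; Damage updates the HUD and triggers shake or explosive death, with PlayerState handling respawn on destruction; ramming deals damage equal to current Health.
; Pickups adjust health and top guns, forwarding lives to PlayerState and fire upgrades to the controller.
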(event `/Game/Core/BPI_MyFlyingShmup.SetPlayerHealth`
  (params (Health :type "Float (double-precision)"))
  ; AnyDamage + Health
  (bind _playerui (message `/Game/Core/BPI_MyFlyingShmup.GetPlayerUi` (`PlayerController.GetHUD` (`self.AsPlayer Controller My Flying Shmup`))))
  (message `/Game/Core/BPI_MyFlyingShmup.SetHealthAsPercent` _playerui (/ (`self.Health`) (`self.MaxHealth`)))
  (if (== (`self.Health`) 0.0)
    (`self.Death`)
    (else
      (`self.HitSequence`))))

(event `self.ReceiveActorBeginOverlap`
  (params (OtherActor :type "Actor Object Reference"))
  ; Collision
  (`GameplayStatics.ApplyDamage` OtherActor (`self.Health`)))

(event `self.ReceiveAnyDamage`
  (params (Damage :type "Float (single-precision)") (DamageType :type "DamageType Object Reference") (InstigatedBy :type "Controller Object Reference") (DamageCauser :type "Actor Object Reference"))
  ; AnyDamage + Health
  (bind _output_get (set `self.Health` (`KismetMathLibrary.FMax` (- (`self.Health`) Damage))))
  (`/Game/Core/BPI_MyFlyingShmup.SetPlayerHealth` _output_get))

(event `Death`
  ; DeathSequence
  (`|ExecutionSequence`
    (:`then_0`
      (`|SpawnActorFromClass` "/Game/Particles/BP_Explosion.BP_Explosion_C" (`KismetMathLibrary.MakeTransform` (`self.K2_GetActorLocation`)) "Undefined" "MultiplyWithRoot" null null)
      (`PlayerController.ClientStartCameraShake` :`self` (`self.AsPlayer Controller My Flying Shmup`) :`Shake` "/Game/Blueprints/BP_CameraShake.BP_CameraShake_C" :`Scale` 3.0)
      (`GameplayStatics.PlaySound2D` "/Game/Sounds/617043__d4xx__bass-impact-3.617043__d4xx__bass-impact-3" 1.0 (`KismetMathLibrary.RandomFloatInRange` 0.5 1.5) 0.0 null null))
    (:`then_2`
      (bind _playerui (message `/Game/Core/BPI_MyFlyingShmup.GetPlayerUi` (`PlayerController.GetHUD` (`self.AsPlayer Controller My Flying Shmup`))))
      (message `/Game/Core/BPI_MyFlyingShmup.PlayScreenFlash` _playerui)
      (`self.SetActorHiddenInGame` true)
      (set `PrimitiveComponent.bGenerateOverlapEvents` false (`self.Box`))
      (`self.DisableInput` (`self.AsPlayer Controller My Flying Shmup`))
      (`self.K2_DestroyActor`))))

(event `HitSequence`
  ; HitSequence
  (`|ExecutionSequence`
    (:`then_0`
      (`PlayerController.ClientStartCameraShake` :`self` (`self.AsPlayer Controller My Flying Shmup`) :`Shake` "/Game/Blueprints/BP_CameraShake.BP_CameraShake_C"))))

(event `self.ReceiveEndPlay`
  (params (EndPlayReason :type "EEndPlayReason Enum" :default "Destroyed"))
  ; SpawnSequence
  (switch `EEndPlayReason` EndPlayReason
    (:`Destroyed`
      (message `/Game/Core/BPI_MyFlyingShmup.RespawnPlayerPawn` (`GameplayStatics.GetPlayerState` 0) (`GameplayStatics.GetObjectClass` self)))))

(event `EnhancedInput|/Game/Inputs/IA_PrimaryFire`
  (params (ActionValue :type Boolean) (ElapsedSeconds :type "Float (double-precision)") (TriggeredSeconds :type "Float (double-precision)") (InputAction :type "InputAction Object Reference" :default "/Game/Inputs/IA_PrimaryFire.IA_PrimaryFire"))
  ; ShootingMode
  (:`Triggered`
    (bind _asplayer_controller_my_flying_shmup (`self.AsPlayer Controller My Flying Shmup`)
      (:`then`
        (set `self.ShootingMode` (`/Game/Core/PlayerControllerMyFlyingShmup.ShootingMode` _asplayer_controller_my_flying_shmup))
        (set `self.SimulBulletsToShoot` (`/Game/Core/PlayerControllerMyFlyingShmup.SimulBulletsToShoot` _asplayer_controller_my_flying_shmup))
        (set `self.ShootingDirection` (`/Game/Core/PlayerControllerMyFlyingShmup.ShootingDirection` _asplayer_controller_my_flying_shmup))
        (set `self.RateOfBulletFire` (`/Game/Core/PlayerControllerMyFlyingShmup.RateOfBulletFire` _asplayer_controller_my_flying_shmup))
        (switch `int` (`self.ShootingMode`)
          (:`0`
            ; RateOfFire
            (`/Engine/EditorBlueprintResources/StandardMacros.DoOnce` false :!label _label
              (:`Completed`
                (`|ExecutionSequence`
                  (:`then_0`
                    ; SimulBullets
                    (for _index (range 1 (+ (`self.SimulBulletsToShoot`) 1))
                      (switch `int` _index
                        (:`1`
                          _)
                        (:`2`
                          (`KismetSystemLibrary.Delay` 0.1))
                        (:`3`
                          (`KismetSystemLibrary.Delay` 0.2)))
                      ; ShootingDirection
                      (for _index_2 (range 1 (+ (`self.ShootingDirection`) 1))
                        (switch `int` _index_2
                          (:`1`
                            (`self.FireSingleBullet` 0.0))
                          (:`2`
                            (`self.FireSingleBullet` 2.0))
                          (:`3`
                            (`self.FireSingleBullet` 3.0))))))
                  (:`then_1`
                    (`KismetSystemLibrary.Delay` (`self.RateOfBulletFire`))
                    (goto _label :!via `Reset`))))))))
      (:`else`))))

(event `SpawnSequence`
  ; SpawnSequence
  (`PrimitiveComponent.SetCollisionEnabled` (`self.Box`) "NoCollision")
  (`MeshComponent.SetOverlayMaterial` (`self.StaticMesh`) "/Game/Materials/M_OverlayMaterial.M_OverlayMaterial"))

(event `self.ReceiveBeginPlay`
  ; SpawnSequence
  (`self.SpawnSequence`)
  (set `self.Health` (`self.MaxHealth`))
  (bind _playerui (message `/Game/Core/BPI_MyFlyingShmup.GetPlayerUi` (`PlayerController.GetHUD` (`GameplayStatics.GetPlayerController` 0))))
  (message `/Game/Core/BPI_MyFlyingShmup.SetHealthAsPercent` _playerui 1.0)
  (`KismetSystemLibrary.Delay` 3.0)
  (set `PrimitiveComponent.bGenerateOverlapEvents` true (`self.Box`))
  (`PrimitiveComponent.SetCollisionEnabled` (`self.Box`) "QueryAndPhysics")
  (`MeshComponent.SetOverlayMaterial` (`self.StaticMesh`) null))

(event `self.ReceiveTick`
  (params (DeltaSeconds :type "Float (single-precision)")))

(event `self.ReceivePossessed`
  (params (NewController :type "Controller Object Reference"))
  ; Adds Input Mapping context for the Owning Controller, if it is a player controller
  (`KismetSystemLibrary.Delay` 2.0)
  (bind _asplayer_controller_my_flying_shmup (cast `/Game/Core/PlayerControllerMyFlyingShmup` NewController))
  (set `self.AsPlayer Controller My Flying Shmup` _asplayer_controller_my_flying_shmup)
  (`EnhancedInputSubsystemInterface.AddMappingContext` (pcsubsystem `EnhancedInputLocalPlayerSubsystem` _asplayer_controller_my_flying_shmup) "/Game/Inputs/IMC_Hero.IMC_Hero" 0 (struct)))

(event `FireSingleBullet`
  (params (RelativeAngle :type "Float (double-precision)") (RelativeLocation :type "Vector Structure"))
  (bind _returnvalue (`self.GetLocalViewingPlayerController`))
  (bind _returnvalue_2 (`KismetMathLibrary.MakeRotator` 0.0 RelativeAngle))
  (bind _topleftgun (`self.TopLeftGun`))
  (bind _toprightgun (`self.TopRightGun`))
  (bind _leftprimaryfire (`self.LeftPrimaryFire`))
  (bind _rightprimaryfire (`self.RightPrimaryFire`))
  ; Spawn2DBullet
  (`|ExecutionSequence`
    (:`then_0`
      (`GameplayStatics.PlaySound2D` "/Game/Sounds/blaster-firing.blaster-firing" 0.1 1.0 0.0 null null false)
      (`|SpawnActorFromClass` "/Game/Blueprints/Player/BP_PlayerFire_Projectile_Bullet.BP_PlayerFire_Projectile_Bullet_C" (`KismetMathLibrary.MakeTransform` (+ RelativeLocation (`SceneComponent.K2_GetComponentLocation` _leftprimaryfire)) (`KismetMathLibrary.ComposeRotators` _returnvalue_2 (`SceneComponent.K2_GetComponentRotation` _leftprimaryfire))) "AlwaysSpawn" "MultiplyWithRoot" _returnvalue 0.0 0.0 self))
    (:`then_1`
      (`|SpawnActorFromClass` "/Game/Blueprints/Player/BP_PlayerFire_Projectile_Bullet.BP_PlayerFire_Projectile_Bullet_C" (`KismetMathLibrary.MakeTransform` (+ RelativeLocation (`SceneComponent.K2_GetComponentLocation` _rightprimaryfire)) (`KismetMathLibrary.ComposeRotators` _returnvalue_2 (`SceneComponent.K2_GetComponentRotation` _rightprimaryfire))) "AlwaysSpawn" "MultiplyWithRoot" _returnvalue 0.0 0.0 self))
    (:`then_2`
      (if (`self.HasTopGuns`)
        (`|SpawnActorFromClass` "/Game/Blueprints/Player/BP_PlayerFire_Projectile_Bullet.BP_PlayerFire_Projectile_Bullet_C" (`KismetMathLibrary.MakeTransform` (+ RelativeLocation (`SceneComponent.K2_GetComponentLocation` _topleftgun)) (`KismetMathLibrary.ComposeRotators` _returnvalue_2 (`SceneComponent.K2_GetComponentRotation` _topleftgun))) "AlwaysSpawn" "MultiplyWithRoot" _returnvalue 0.0 0.0 self)))
    (:`then_3`
      (if (`self.HasTopGuns`)
        (`|SpawnActorFromClass` "/Game/Blueprints/Player/BP_PlayerFire_Projectile_Bullet.BP_PlayerFire_Projectile_Bullet_C" (`KismetMathLibrary.MakeTransform` (+ RelativeLocation (`SceneComponent.K2_GetComponentLocation` _toprightgun)) (`KismetMathLibrary.ComposeRotators` _returnvalue_2 (`SceneComponent.K2_GetComponentRotation` _toprightgun))) "AlwaysSpawn" "MultiplyWithRoot" _returnvalue 0.0 0.0 self)))))

(event `/Game/Core/BPI_MyFlyingShmup.OnCollectPickUp`
  (params (MaxHealth :type "Float (double-precision)") (Health :type "Float (double-precision)") (Lives :type Integer) (GlobalEnemyDamage :type "Float (double-precision)") (RateOfFire :type "Float (double-precision)") (ShootingDirection :type Integer) (HasTopGuns :type Boolean) (SimulBulletstoShoot :type Integer))
  ; Pickups
  (`|ExecutionSequence`
    (:`then_0`
      (set `self.MaxHealth` (`KismetMathLibrary.FMax` (+ (`self.MaxHealth`) MaxHealth)))
      (`/Game/Core/BPI_MyFlyingShmup.SetPlayerHealth` (`self.Health`)))
    (:`then_1`
      (bind _output_get (set `self.Health` (`KismetMathLibrary.FMax` (+ (`self.Health`) Health))))
      (`/Game/Core/BPI_MyFlyingShmup.SetPlayerHealth` _output_get))
    (:`then_2`
      (message `/Game/Core/BPI_MyFlyingShmup.AddPlayerLife` (`Controller.PlayerState` (`self.GetController`)) Lives))
    (:`then_3`
      (set `self.HasTopGuns` HasTopGuns)
      (`KismetSystemLibrary.K2_SetTimerDelegate` (delegate `DisableTopGuns`) 45.0))
    (:`then_4`
      (message `/Game/Core/BPI_MyFlyingShmup.OnCollectPickUp` (`self.GetController`) 0.0 0.0 0 0.0 RateOfFire ShootingDirection false SimulBulletstoShoot))))

(event `EnhancedInput|/Game/Inputs/IA_MoveForwardBackwards`
  (params (ActionValue :type "Float (double-precision)") (ElapsedSeconds :type "Float (double-precision)") (TriggeredSeconds :type "Float (double-precision)") (InputAction :type "InputAction Object Reference" :default "/Game/Inputs/IA_MoveForwardBackwards.IA_MoveForwardBackwards"))
  ; Movement
  (:`Triggered`
    (`PawnMovementComponent.AddInputVector` (`self.FloatingPawnMovement`) (`KismetMathLibrary.MakeVector` 0.0 0.0 ActionValue) false)))

(event `EnhancedInput|/Game/Inputs/IA_RotationDown`
  (params (ActionValue :type Boolean) (ElapsedSeconds :type "Float (double-precision)") (TriggeredSeconds :type "Float (double-precision)") (InputAction :type "InputAction Object Reference" :default "/Game/Inputs/IA_RotationDown.IA_RotationDown"))
  (bind _staticmesh (`self.StaticMesh`))
  ; Ship Rotation
  (:`Triggered`
    (`SceneComponent.K2_SetRelativeRotation` _staticmesh (struct :`Pitch` -20.0) false false))
  (:`Completed`
    (`SceneComponent.K2_SetRelativeRotation` :`self` _staticmesh)))

(event `EnhancedInput|/Game/Inputs/IA_RotationUp`
  (params (ActionValue :type Boolean) (ElapsedSeconds :type "Float (double-precision)") (TriggeredSeconds :type "Float (double-precision)") (InputAction :type "InputAction Object Reference" :default "/Game/Inputs/IA_RotationUp.IA_RotationUp"))
  (bind _staticmesh (`self.StaticMesh`))
  ; Ship Rotation
  (:`Triggered`
    (`SceneComponent.K2_SetRelativeRotation` _staticmesh (struct :`Pitch` 20.0) false false))
  (:`Completed`
    (`SceneComponent.K2_SetRelativeRotation` :`self` _staticmesh)))

(event `EnhancedInput|/Game/Inputs/IA_MoveRightLeft`
  (params (ActionValue :type "Float (double-precision)") (ElapsedSeconds :type "Float (double-precision)") (TriggeredSeconds :type "Float (double-precision)") (InputAction :type "InputAction Object Reference" :default "/Game/Inputs/IA_MoveRightLeft.IA_MoveRightLeft"))
  ; Movement
  (:`Triggered`
    (`PawnMovementComponent.AddInputVector` (`self.FloatingPawnMovement`) (`KismetMathLibrary.MakeVector` 0.0 ActionValue) false)))

(event `DisableTopGuns`
  ; Pickups
  (set `self.HasTopGuns` false))

(fn `AddPlayerLife`
  (params (LivesToAdd :type Integer))
  (returns (LivesRemaining :type Integer))
  (return 0))

(fn `GetPlayerUi`
  (returns (PlayerUi :type "UserWidget Object Reference"))
  (return null))

(fn `SetHealthAsPercent`
  (params (Percent :type "Float (double-precision)")))

(fn `UserConstructionScript`)