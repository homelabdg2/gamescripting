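; BP_Bullet is a player bullet actor driven by a ProjectileMovement component.
; On BeginPlay it sets the component's InitialSpeed to Speed times SpeedMultiplier and matches MaxSpeed to that value.
; The graph holds no hit or damage logic: overlap and Tick are disabled stubs, the parent BeginPlay call is unwired, and the construction script only calls its parent.
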(event `self.ReceiveBeginPlay`
  (bind _projectilemovement (`self.ProjectileMovement`))
  (bind _output_get (set `ProjectileMovementComponent.InitialSpeed` (* (`self.Speed`) (`self.SpeedMultiplier`)) _projectilemovement))
  (set `ProjectileMovementComponent.MaxSpeed` _output_get _projectilemovement))

(fn `UserConstructionScript`
  (`parent.UserConstructionScript`))