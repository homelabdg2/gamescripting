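; Enemy actor that damages the hero on overlap by its current Health and awards its MaxHealth as score when killed.
; Damage lowers Health, updates the widget health bar, and either briefly applies an overlay material or triggers Death.
; Death plays a pitch-randomized sound, spawns an explosion, score actor and configurable pickup, then adds score and destroys itself.
; A Z-clamp helper and several empty stub functions are unused in these graphs.
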(event `self.ReceiveActorBeginOverlap`
  (params (OtherActor :type "Actor Object Reference"))
  ; Apply damage to player on collision
  (cast `/Game/Blueprints/Player/BP_Hero` OtherActor)
  (`GameplayStatics.ApplyDamage` OtherActor (`self.Health`)))

(event `self.ReceiveAnyDamage`
  (params (Damage :type "Float (single-precision)") (DamageType :type "DamageType Object Reference") (InstigatedBy :type "Controller Object Reference") (DamageCauser :type "Actor Object Reference"))
  ; Enemy health system
  (bind _output_get (set `self.Health` (`KismetMathLibrary.FMax` (- (`self.Health`) Damage))))
  (`/Game/Ui/WBP_EnemyHealthBar.SetHealthBarByPercent` (`self.HealthBar`) (/ (`self.Health`) (`self.MaxHealth`)))
  (if (<= _output_get 0.0)
    (`self.Death`)
    (else
      (`MeshComponent.SetOverlayMaterial` (`self.StaticMesh`) "/Game/Materials/M_OverlayMaterial.M_OverlayMaterial")
      (`KismetSystemLibrary.Delay` 1.0)
      (`MeshComponent.SetOverlayMaterial` (`self.StaticMesh`) null))))

(event `self.ReceiveBeginPlay`
  ; Enemy Healthbar
  (bind _aswbp_enemy_health_bar (cast `/Game/Ui/WBP_EnemyHealthBar` (`WidgetComponent.GetWidget` (`self.Widget`))))
  (set `self.HealthBar` _aswbp_enemy_health_bar))

(event `Death`
  (bind _returnvalue (`self.K2_GetActorLocation`))
  ; Death Sequence
  (`|ExecutionSequence`
    (:`then_0`
      (`GameplayStatics.PlaySound2D` "/Game/Sounds/617043__d4xx__bass-impact-3.617043__d4xx__bass-impact-3" 0.5 (`KismetMathLibrary.RandomFloatInRange` 0.5 1.5) 0.0 null null))
    (:`then_1`
      (`|SpawnActorFromClass` "/Game/Particles/BP_Explosion.BP_Explosion_C" (`KismetMathLibrary.MakeTransform` _returnvalue) "Undefined" "MultiplyWithRoot" null null)
      (`|SpawnActorFromClass` "/Game/Blueprints/Enemies/BP_KillScore.BP_KillScore_C" (`KismetMathLibrary.MakeTransform` _returnvalue) "AlwaysSpawn" "MultiplyWithRoot" null (`self.MaxHealth`) null)
      (`|SpawnActorFromClass` (`self.PickUpToDropOnDeath`) (`self.GetTransform`) "Undefined" "MultiplyWithRoot" null null))
    (:`then_2`
      (bind _asbp_hero (cast `/Game/Blueprints/Player/BP_Hero` (`GameplayStatics.GetPlayerPawn` 0)))
      (set `/Game/Blueprints/Player/BP_Hero.Score` (+ (`/Game/Blueprints/Player/BP_Hero.Score` _asbp_hero) (`self.MaxHealth`)) _asbp_hero)
      (`self.K2_DestroyActor`))))

(event `/Game/Core/BPI_MyFlyingShmup.SetPickupToDropOnDeath`
  (params (PickUpClass :type "/Game/Blueprints/Player/BP_Pickup Class Reference"))
  (set `self.PickUpToDropOnDeath` PickUpClass))

(fn `AddPlayerLife`
  (params (LivesToAdd :type Integer))
  (returns (LivesRemaining :type Integer))
  (return 0))

(fn `ClampMovement`
  (params (MovementDelta :type "Vector Structure"))
  (returns (ReturnValue :type "Vector Structure"))
  (bind _z (.z (`self.K2_GetActorLocation`)))
  ; Clamp movement
  (return (`KismetMathLibrary.MakeVector` (.x (`self.K2_GetActorLocation`)) (.y (`self.K2_GetActorLocation`)) (- _z (`KismetMathLibrary.FClamp` (+ _z (.z MovementDelta)) (`self.MinZ`) (`self.MaxZ`))))))

(fn `GetPlayerUi`
  (returns (PlayerUi :type "UserWidget Object Reference"))
  (return null))

(fn `SetHealthAsPercent`
  (params (Percent :type "Float (double-precision)"))
  (returns (Return :type Boolean))
  (return false))

(fn `UserConstructionScript`)