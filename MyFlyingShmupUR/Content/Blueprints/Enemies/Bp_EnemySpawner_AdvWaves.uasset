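; Enemy spawner that runs the game through data-driven waves, playing boss music on boss waves and showing the win screen after the last one.
; Chained events step through waves, enemy groups and individual timed spawns, polling until no enemies remain before starting the next group.
; A random stream sets each spawn's height between the Up and Down markers and gives some enemies a random pickup to drop on death.
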(event `self.ReceiveBeginPlay`
  (set `self.CurrentWaveIndex` -1)
  (`self.NextWave`))

(event `NextWave`
  (`KismetSystemLibrary.PrintString` "NextWave")
  (`/Engine/EditorBlueprintResources/StandardMacros.IncrementInt` (`self.CurrentWaveIndex`)
    (:`  `
      (if (`KismetArrayLibrary.Array_IsValidIndex` (`self.WaveData`) (`self.CurrentWaveIndex`))
        (bind _output_get (set `self.CurrentWave` (`|GetArrayItem` (`self.WaveData`) (`self.CurrentWaveIndex`))))
        (if (`.IsBossWave_10_9FCD956A4CC5BF199DC8EA9442BF4973` (break `/Game/Core/S_wave` _output_get))
          (`GameplayStatics.PlaySound2D` "/Game/Sounds/imperial_march.imperial_march" 1.0 1.0 0.0 null null))
        (`KismetSystemLibrary.Delay` (`.InitialDelay_5_D33052934AD4F93442FF7DA37033733A` (break `/Game/Core/S_wave` _output_get)))
        (set `self.EnemiesIndex` -1)
        (`self.SpawnNextEnemyGroup`)
        (else
          (`KismetSystemLibrary.PrintString` "GameWinScreen")
          (message `/Game/Core/BPI_MyFlyingShmup.ShowEndScreen` (`PlayerController.GetHUD` (`GameplayStatics.GetPlayerController` 0)) true))))))

(event `SpawnNextEnemyGroup`
  (bind (_currentwave_waveid _currentwave_initialdelay _currentwave_frequency _currentwave_isbosswave _currentwave_enemies) (break `/Game/Core/S_wave` (`self.CurrentWave`)))
  (bind (_output_enemyclass _output_numbertospawn) (break `/Game/Core/S_EnemyAndCount` (`|GetArrayItem` (`self.CurrentWaveCurrentEnemies`) (`self.EnemiesIndex`))))
  (`KismetSystemLibrary.PrintString` "SpawnNextEnemyGroup")
  (`/Engine/EditorBlueprintResources/StandardMacros.IncrementInt` (`self.EnemiesIndex`)
    (:`  `
      (bind _output_get (set `self.CurrentWaveCurrentEnemies` _currentwave_enemies))
      (if (`KismetArrayLibrary.Array_IsValidIndex` _output_get (`self.EnemiesIndex`))
        (set `self.EnemyClassToSpawn` _output_enemyclass)
        (set `self.EnemiesRemaining` _output_numbertospawn)
        (`self.SpawnNextEnemyInCurrentGroup`)
        (else
          (`self.NextWave`))))))

(event `SpawnNextEnemyInCurrentGroup`
  (bind (_currentwave_waveid _currentwave_initialdelay _currentwave_frequency) (break `/Game/Core/S_wave` (`self.CurrentWave`)))
  (if (> (`self.EnemiesRemaining`) 0)
    (`/Engine/EditorBlueprintResources/StandardMacros.DecrementInt` (`self.EnemiesRemaining`)
      (:`  `
        (bind _returnvalue (`KismetSystemLibrary.K2_SetTimerDelegate` (delegate `SpawnEnemy`) _currentwave_frequency))
        (set `self.WaveTimer` _returnvalue)
        (`KismetSystemLibrary.PrintString` "SpawnEnemy")))
    (else
      (`self.CheckIfCurrentEnemyGroupIsDead`)
      (`self.SpawnNextEnemyGroup`))))

(event `SpawnEnemy`
  (bind (_returnvalue_x _returnvalue_y _returnvalue_z) (`KismetMathLibrary.BreakVector` (`SceneComponent.K2_GetComponentLocation` (`self.Up`))))
  (bind (_returnvalue_x_2 _returnvalue_y_2 _returnvalue_z_2) (`KismetMathLibrary.BreakVector` (`SceneComponent.K2_GetComponentLocation` (`self.Down`))))
  (`KismetSystemLibrary.PrintString` "SpawningEnemy")
  (`self.SpawnNextEnemyInCurrentGroup`)
  (bind _returnvalue (`|SpawnActorFromClass` (`self.EnemyClassToSpawn`) (`KismetMathLibrary.MakeTransform` (`KismetMathLibrary.MakeVector` 0.0 _returnvalue_y (`KismetMathLibrary.RandomFloatInRangeFromStream` (`self.Stream`) (`KismetMathLibrary.FMin` _returnvalue_z _returnvalue_z_2) (`KismetMathLibrary.FMax` _returnvalue_z _returnvalue_z_2))) (`SceneComponent.K2_GetComponentRotation` (`self.Down`))) "Undefined" "MultiplyWithRoot" null null))
  (if (`KismetMathLibrary.RandomBoolWithWeightFromStream` (`self.Stream`) 0.33)
    (message `/Game/Core/BPI_MyFlyingShmup.SetPickupToDropOnDeath` _returnvalue (`KismetArrayLibrary.Array_RandomFromStream` (`|MakeArray` "/Game/Blueprints/Player/BP_Pickup_Spread.BP_Pickup_Spread_C" "/Game/Blueprints/Player/BP_Pickup_Lives.BP_Pickup_Lives_C" "/Game/Blueprints/Player/BP_Pickup_Rate+TopGuns.BP_Pickup_Rate+TopGuns_C" :!type "/Game/Blueprints/Player/BP_Pickup Class Reference") (`self.Stream`)))))

(fn `UserConstructionScript`)