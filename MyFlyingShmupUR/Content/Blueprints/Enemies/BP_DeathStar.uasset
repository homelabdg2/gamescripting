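; BP_DeathStar is an enemy Blueprint that fires bullets at the player.
; On BeginPlay it calls the parent logic, then starts a looping timer that runs ShootBullet every 0.6 seconds.
; Each shot spawns two Bp_EnemyFire_Bullet actors from the Arrow and Arrow1 components, each rotated to face player pawn 0's position at spawn time.
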(event `self.ReceiveBeginPlay`
  (`parent.ReceiveBeginPlay`)
  (`KismetSystemLibrary.K2_SetTimerDelegate` (delegate `ShootBullet`) 0.6 true true))

(event `ShootBullet`
  (bind _returnvalue (`SceneComponent.K2_GetComponentLocation` (`self.Arrow1`)))
  (bind _returnvalue_2 (`SceneComponent.K2_GetComponentLocation` (`self.Arrow`)))
  (`|SpawnActorFromClass` "/Game/Blueprints/Enemies/Bp_EnemyFire_Bullet.Bp_EnemyFire_Bullet_C" (`KismetMathLibrary.MakeTransform` _returnvalue_2 (`KismetMathLibrary.FindLookAtRotation` _returnvalue_2 (`self.K2_GetActorLocation` (`GameplayStatics.GetPlayerPawn` 0)))) "Undefined" "MultiplyWithRoot" null null)
  (`|SpawnActorFromClass` "/Game/Blueprints/Enemies/Bp_EnemyFire_Bullet.Bp_EnemyFire_Bullet_C" (`KismetMathLibrary.MakeTransform` _returnvalue (`KismetMathLibrary.FindLookAtRotation` _returnvalue (`self.K2_GetActorLocation` (`GameplayStatics.GetPlayerPawn` 0)))) "Undefined" "MultiplyWithRoot" null null))

(fn `UserConstructionScript`)