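; Simple enemy spawner that periodically creates one of two enemy Blueprints on a looping timer started at BeginPlay.
; Each spawn lands at X zero on the Up component's Y, at a random Z between the Up and Down markers, using Down's rotation.
; About a third of spawns receive a random pickup to drop on death, with all random choices drawn from a random stream.
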(event `self.ReceiveBeginPlay`
  (`KismetSystemLibrary.K2_SetTimerDelegate` (delegate `SpawnEnemy`) 6.0 true true))

(event `SpawnEnemy`
  (bind _stream (`self.Stream`))
  (bind (_returnvalue_x _returnvalue_y _returnvalue_z) (`KismetMathLibrary.BreakVector` (`SceneComponent.K2_GetComponentLocation` (`self.Up`))))
  (bind (_returnvalue_x_2 _returnvalue_y_2 _returnvalue_z_2) (`KismetMathLibrary.BreakVector` (`SceneComponent.K2_GetComponentLocation` (`self.Down`))))
  (bind _returnvalue (`|SpawnActorFromClass` (`KismetArrayLibrary.Array_RandomFromStream` (`|MakeArray` "/Game/Blueprints/Enemies/Bp_Enemy_E.Bp_Enemy_E_C" "/Game/Blueprints/Enemies/Bp_Enemy_D.Bp_Enemy_D_C" :!type "Actor Class Reference") _stream) (`KismetMathLibrary.MakeTransform` (`KismetMathLibrary.MakeVector` 0.0 _returnvalue_y (`KismetMathLibrary.RandomFloatInRangeFromStream` _stream (`KismetMathLibrary.FMin` _returnvalue_z _returnvalue_z_2) (`KismetMathLibrary.FMax` _returnvalue_z _returnvalue_z_2))) (`SceneComponent.K2_GetComponentRotation` (`self.Down`))) "Undefined" "MultiplyWithRoot" null null))
  (if (`KismetMathLibrary.RandomBoolWithWeightFromStream` (`self.Stream`) 0.33)
    (message `/Game/Core/BPI_MyFlyingShmup.SetPickupToDropOnDeath` _returnvalue (`KismetArrayLibrary.Array_RandomFromStream` (`|MakeArray` "/Game/Blueprints/Player/BP_Pickup_Spread.BP_Pickup_Spread_C" "/Game/Blueprints/Player/BP_Pickup_Lives.BP_Pickup_Lives_C" "/Game/Blueprints/Player/BP_Pickup_Rate+TopGuns.BP_Pickup_Rate+TopGuns_C" :!type "/Game/Blueprints/Player/BP_Pickup Class Reference") (`self.Stream`)))))

(fn `UserConstructionScript`)