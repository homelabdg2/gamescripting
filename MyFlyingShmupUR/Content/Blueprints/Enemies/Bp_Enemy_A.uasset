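; Enemy actor that homes in on player 0's pawn along a weaving path.
; Each Tick it normalizes the direction to the pawn, scales it by Speed and delta time, and adds a sine offset on world Y driven by accumulated RunningTime, WaveFrequency and WaveAmplitude.
; The wave term is applied per frame without delta scaling, so its sway depends on frame rate, and movement does not sweep for collision.
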(event `self.ReceiveTick`
  (params (DeltaSeconds :type "Float (single-precision)"))
  ; Movement
  (bind _returnvalue (`GameplayStatics.GetPlayerPawn` 0))
  (if (`KismetSystemLibrary.IsValid` _returnvalue)
    (bind _returnvalue_2 (`self.K2_GetActorLocation` _returnvalue))
    (bind _output_get (set `self.RunningTime` (+ DeltaSeconds (`self.RunningTime`))))
    (`self.K2_AddActorWorldOffset` (+ (`KismetMathLibrary.MakeVector` 0.0 (* (* (`KismetMathLibrary.DegSin` (* _output_get (`self.WaveFrequency`))) (`self.WaveAmplitude`)) -1.0)) (* (* (`KismetMathLibrary.Normal` (- (`self.K2_GetActorLocation`) _returnvalue_2)) -1.0) (* (`self.Speed`) DeltaSeconds))))))

(event `Offset`)

(fn `UserConstructionScript`
  (`parent.UserConstructionScript`))