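; Turret enemy Blueprint that periodically fires bullets at the player.
; On BeginPlay, after calling the parent, it starts a looping two-second timer that triggers ShootBullet.
; Each shot spawns an enemy bullet at the Arrow component's location, rotated toward the first player pawn's current position via FindLookAtRotation.
; The turret itself never rotates; only the spawned projectile is aimed.
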(event `self.ReceiveBeginPlay`
  (`parent.ReceiveBeginPlay`)
  (`KismetSystemLibrary.K2_SetTimerDelegate` (delegate `ShootBullet`) 2.0 true true))

(event `ShootBullet`
  (bind _returnvalue (`SceneComponent.K2_GetComponentLocation` (`self.Arrow`)))
  (`|SpawnActorFromClass` "/Game/Blueprints/Enemies/Bp_EnemyFire_Bullet.Bp_EnemyFire_Bullet_C" (`KismetMathLibrary.MakeTransform` _returnvalue (`KismetMathLibrary.FindLookAtRotation` _returnvalue (`self.K2_GetActorLocation` (`GameplayStatics.GetPlayerPawn` 0)))) "Undefined" "MultiplyWithRoot" null null))

(fn `UserConstructionScript`
  (`parent.UserConstructionScript`))