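; Simple enemy spawner actor that spawns a Bp_Enemy_B at a regular interval.
; A looping timer started on BeginPlay fires SpawnEnemy, which picks from a single-entry class array and prints a debug message.
; The Up and Down components bound a random spawn height, with X fixed at zero, Y taken from Up and rotation from Down.
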(event `self.ReceiveBeginPlay`
  (`KismetSystemLibrary.K2_SetTimerDelegate` (delegate `SpawnEnemy`) 2.0 true true))

(event `SpawnEnemy`
  (bind (_returnvalue_x _returnvalue_y _returnvalue_z) (`KismetMathLibrary.BreakVector` (`SceneComponent.K2_GetComponentLocation` (`self.Up`))))
  (bind (_returnvalue_x_2 _returnvalue_y_2 _returnvalue_z_2) (`KismetMathLibrary.BreakVector` (`SceneComponent.K2_GetComponentLocation` (`self.Down`))))
  (`|SpawnActorFromClass` (`KismetArrayLibrary.Array_Random` (`|MakeArray` "/Game/Blueprints/Enemies/Bp_Enemy_B.Bp_Enemy_B_C" :!type "Actor Class Reference")) (`KismetMathLibrary.MakeTransform` (`KismetMathLibrary.MakeVector` 0.0 _returnvalue_y (`KismetMathLibrary.RandomFloatInRange` (`KismetMathLibrary.FMin` _returnvalue_z _returnvalue_z_2) (`KismetMathLibrary.FMax` _returnvalue_z _returnvalue_z_2))) (`SceneComponent.K2_GetComponentRotation` (`self.Down`))) "Undefined" "MultiplyWithRoot" null null)
  (`KismetSystemLibrary.PrintString` "Spawned"))

(fn `UserConstructionScript`)