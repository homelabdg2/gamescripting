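; Enemy B is an enemy that flies a wavy zigzag path while firing bullets on a looping timer.
; Tick moves it steadily along negative Y without sweep, while a sine of accumulated running time offsets Z around the height stored at BeginPlay.
; After calling the parent BeginPlay, it starts the timer that spawns Bp_EnemyFire_Bullet at the Arrow component's location and rotation.
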(event `self.ReceiveTick`
  (params (DeltaSeconds :type "Float (single-precision)"))
  (bind (_returnvalue_x _returnvalue_y) (`KismetMathLibrary.BreakVector` (`self.K2_GetActorLocation`)))
  ; ZigZag Movement
  (bind _output_get (set `self.RunningTime` (+ DeltaSeconds (`self.RunningTime`))))
  (`self.K2_SetActorLocation` (`KismetMathLibrary.MakeVector` _returnvalue_x (+ _returnvalue_y (* (`self.Speed`) (`GameplayStatics.GetWorldDeltaSeconds`) -1.0)) (+ (* (`KismetMathLibrary.DegSin` (* _output_get (`self.WaveFrequency`))) (`self.WaveAmplitude`)) (`self.StartZ`)))))

(event `self.ReceiveBeginPlay`
  ; Shoot
  (`parent.ReceiveBeginPlay`)
  (`|ExecutionSequence`
    (:`then_0`
      (set `self.StartZ` (.z (`self.K2_GetActorLocation`))))
    (:`then_1`
      (`KismetSystemLibrary.K2_SetTimerDelegate` (delegate `ShootBullet`) 3.0 true true))))

(event `ShootBullet`
  (bind _arrow (`self.Arrow`))
  ; Shoot
  (`|SpawnActorFromClass` "/Game/Blueprints/Enemies/Bp_EnemyFire_Bullet.Bp_EnemyFire_Bullet_C" (`KismetMathLibrary.MakeTransform` (`SceneComponent.K2_GetComponentLocation` _arrow) (`SceneComponent.K2_GetComponentRotation` _arrow)) "Undefined" "MultiplyWithRoot" null null))

(fn `UserConstructionScript`
  (`parent.UserConstructionScript`))